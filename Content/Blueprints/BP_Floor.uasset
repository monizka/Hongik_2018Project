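; BP_Floor is a destructible floor that shatters when a BP_lightbulb touches it and ends the game.
; The lightbulb overlapping its Box trigger applies massive radius damage to the DestructibleComponent.
; The fracture event enables gravity on the component and briefly drops global time dilation for slow motion.
; It then restores normal speed, fades camera and audio out, and quits the game after a delay.
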(event `self.Box.OnComponentBeginOverlap`
  (params (OverlappedComponent :type "PrimitiveComponent Object Reference") (OtherActor :type "Actor Object Reference") (OtherComp :type "PrimitiveComponent Object Reference") (OtherBodyIndex :type Integer) (bFromSweep :type Boolean) (SweepResult :type "HitResult Structure (by ref)"))
  (cast `/Game/Blueprints/BP_lightbulb` OtherActor)
  (`DestructibleComponent.ApplyRadiusDamage` (`self.DestructibleComponent`) 1000000000.0 (0.0 0.0 0.0) 2500.0 5000.0 false))

(event `self.DestructibleComponent.OnComponentFracture`
  (params (HitPoint :type "Vector Structure (by ref)") (HitDirection :type "Vector Structure (by ref)"))
  (`GameplayStatics.SetGlobalTimeDilation` 0.1)
  (`PrimitiveComponent.SetEnableGravity` (`self.DestructibleComponent`) true)
  (`KismetSystemLibrary.Delay` 0.5)
  (`GameplayStatics.SetGlobalTimeDilation` 1.0)
  (`PlayerCameraManager.StartCameraFade` :`self` (`PlayerController.PlayerCameraManager` (`GameplayStatics.GetPlayerController` 0)) :`ToAlpha` 1.0 :`Duration` 3.0 :`bShouldFadeAudio` true :`bHoldWhenFinished` true)
  (`KismetSystemLibrary.Delay` 3.5)
  (`KismetSystemLibrary.QuitGame` null "Quit"))

(fn `UserConstructionScript`)